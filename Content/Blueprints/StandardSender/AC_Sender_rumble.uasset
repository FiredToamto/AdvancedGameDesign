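; Sender component that feeds rumble tracking to actors overlapping its owner.
; On BeginPlay it binds to the owner's begin and end overlap events.
; On entry it turns on tracking in the other actor's AC_Reciver_Rumble component and passes the owner's location once, with a zero dial signal.
; On exit it turns tracking off; both events print debug strings.
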(event `self.ReceiveBeginPlay`
  (add `Actor.OnActorBeginOverlap` (`self.GetOwner`) (delegate `OverlapBegin`))
  (add `Actor.OnActorEndOverlap` (`self.GetOwner`) (delegate `OverlapEnd`)))

(event `OverlapBegin`
  (params (OverlappedActor :type "Actor Object Reference") (OtherActor :type "Actor Object Reference"))
  (bind _returnvalue (`Actor.GetComponentByClass` OtherActor "/Game/Blueprints/StandardReciver/AC_Reciver_Rumble.AC_Reciver_Rumble_C"))
  (message `/Game/Blueprints/StandardReciver/BI_Reciver.SetTracking` _returnvalue true)
  (message `/Game/Blueprints/StandardReciver/BI_Reciver.SetTrackedObjectPos` _returnvalue (`Actor.K2_GetActorLocation` (`self.GetOwner`)) 0)
  (`KismetSystemLibrary.PrintString` "InRadius"))

(event `OverlapEnd`
  (params (OverlappedActor :type "Actor Object Reference") (OtherActor :type "Actor Object Reference"))
  (message `/Game/Blueprints/StandardReciver/BI_Reciver.SetTracking` (`Actor.GetComponentByClass` OtherActor "/Game/Blueprints/StandardReciver/AC_Reciver_Rumble.AC_Reciver_Rumble_C") false)
  (`KismetSystemLibrary.PrintString` "OutOfRadius"))