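; Actor component that gives proximity feedback toward a tracked position through beeps and force feedback, fed by external tracking, look and distance events.
; Two self-recalling Delay loops run while tracking: one normalizes owner-to-target distance each frame, the other fires feedback unless not looking.
; Closer range shortens the pulse interval and strengthens rumble.
; Distance uses a fixed divisor, leaving start-distance math unused; light and camera shake are empty stubs.
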(event `/Game/Blueprints/LineTraceReciver/BI_LineTraceReciver.NotLooking`
  (params (IsNotLooking :type Boolean))
  ;[1 1 1] Set is not looking
  (set `self.IsNotLooking` IsNotLooking))

(event `/Game/Blueprints/LineTraceReciver/BI_LineTraceReciver.SendDistance`
  (params (Distance :type "Float (single-precision)"))
  ;[1 0 0.06651] Set actual distance
  (set `self.AcutalDistance` Distance))

(event `/Game/Blueprints/StandardReciver/BI_Reciver.SetTrackedObjectPos`
  (params (ObjectPos :type "Vector Structure") (IsGood :type Boolean))
  ;[1 0.9083 0] Set tracked object position
  (set `self.TrackedObjectPos` ObjectPos))

(event `/Game/Blueprints/StandardReciver/BI_Reciver.SetTracking`
  (params (Tracking :type Boolean))
  ;[0 1 0.006555] Set tracking and start tracking
  (set `self.Tracking` Tracking)
  (`self.StartTracking`))

(event `StartTracking`
  ;[1 0 0.9602] Set tracked position and calculate start distance
  (set `self.StartTrackedPosition` (`Actor.K2_GetActorLocation` (`self.GetOwner`)))
  (set `self.StartDistance` (`KismetMathLibrary.Vector_Distance` (`self.StartTrackedPosition`) (`self.TrackedObjectPos`)))
  ;[0 1 0.9754] Start IsTracking and UpdateDistance
  (`self.IsTracking`)
  (`self.Update Distance`))

(event `IsTracking`
  ;[0 0.04559 1] IsTracking
  (if (`self.Tracking`)
    (if (not (`self.IsNotLooking`))
      ;;[1 0.9238 0.3] Start Actions
      (`self.Play Rumble`)
      (`self.Play Sound`))
    (`KismetSystemLibrary.Delay` (`self.CalculateDelay`))
    (`self.IsTracking`)
    (else
      (set `self.Distance` 1.0))))

(event `Update Distance`
  ;[1 0.6223 0.5322] Update distance and get multiplier
  (if (`self.Tracking`)
    (set `self.Distance` (`self.CalculateDistance`))
    (`self.FF Multiplier`)
    (`KismetSystemLibrary.Delay` (`GameplayStatics.GetWorldDeltaSeconds`))
    (`self.Update Distance`)))

(event `Play Sound`
  ;[0.7759 0.4121 1] Play sound
  (if (`self.CanPlaySound`)
    (`GameplayStatics.PlaySound2D` "/Game/Audio/Detector/Beep3.Beep3" 1.0 1.0 0.0 null null)))

(event `Play Rumble`
  ;[0.4825 1 0.5696] Play rumble
  (if (`self.CanRumble`)
    (`GameplayStatics.SpawnForceFeedbackAtLocation` "/Game/Blueprints/Rumble/FfeTest.FfeTest" (0.0 0.0 0.0) (struct) false (`self.rumbleMulti`) 0.0 null)))

(event `PlayLight`)

(event `Play CameraShake`)

(fn `CalculateDelay`
  (returns (DelayTime :type "Float (double-precision)"))
  ;[1 1 1] Calculate delay based upon distance percentage
  (if (> (`self.Distance`) 0.5)
    (return (+ (`self.Distance`) 0.4))
    (elif (> (`self.Distance`) 0.2)
      (return (+ (`self.Distance`) 0.2))
      (else
        (return (`KismetMathLibrary.FClamp` (`self.Distance`) 0.2))))))

(fn `CalculateDistance`
  (returns (`Distance left in %` :type "Float (double-precision)"))
  ;[1 0 0.1665] If distance isn't closer than start distance
  (return (/ (`KismetMathLibrary.Vector_Distance` (`Actor.K2_GetActorLocation` (`self.GetOwner`)) (`self.TrackedObjectPos`)) 750.0)))

(fn `FF Multiplier`
  ;[1 1 1] Rumble streangt based upon proximity
  (if (>= (`self.Distance`) 0.6)
    (set `self.rumbleMulti` 0.5)
    (elif (>= (`self.Distance`) 0.3)
      (set `self.rumbleMulti` 1.0)
      (elif (>= (`self.Distance`) 0.0)
        (set `self.rumbleMulti` 2.5)))))