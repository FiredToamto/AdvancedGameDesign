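; AC_Sender is an actor component that broadcasts its owner's position and a dial signal to receivers.
; On BeginPlay it binds to the owner's begin and end overlap events.
; Entering overlap sends the owner's location and DialSignal to the other actor's AC_Reciver component, and leaving tells that component to remove the DialSignal entry.
; Both overlap handlers print debug strings.
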(event `self.ReceiveBeginPlay`
  (add `Actor.OnActorBeginOverlap` (`self.GetOwner`) (delegate `OverlapBegin`))
  (add `Actor.OnActorEndOverlap` (`self.GetOwner`) (delegate `OverlapEnd`)))

(event `OverlapBegin`
  (params (OverlappedActor :type "Actor Object Reference") (OtherActor :type "Actor Object Reference"))
  (message `/Game/Blueprints/StandardReciver/BI_Reciver.SetTrackedObjectPos` (`Actor.GetComponentByClass` OtherActor "/Game/Blueprints/StandardReciver/AC_Reciver.AC_Reciver_C") (`Actor.K2_GetActorLocation` (`self.GetOwner`)) (`self.DialSignal`))
  (`KismetSystemLibrary.PrintString` "InRadius"))

(event `OverlapEnd`
  (params (OverlappedActor :type "Actor Object Reference") (OtherActor :type "Actor Object Reference"))
  (message `/Game/Blueprints/StandardReciver/BI_Reciver.RemoveIndex` (`Actor.GetComponentByClass` OtherActor "/Game/Blueprints/StandardReciver/AC_Reciver.AC_Reciver_C") (`self.DialSignal`))
  (`KismetSystemLibrary.PrintString` "OutOfRadius"))