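; Receiver component that acts as a proximity tracker, pulsing feedback as its owner moves toward a tracked position.
; While tracking, it recomputes remaining distance every frame as a fraction of the starting distance, using delay-based self-calling events instead of Tick.
; That fraction is the delay between pulses, so they quicken on approach.
; Each pulse plays a beep and force feedback, and messages the owner to blink its lamp and spin.
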(event `SetActivated`
  (params (SetIsActive :type Boolean))
  (set `self.Activated` SetIsActive))

(event `/Game/Blueprints/StandardReciver/BI_Reciver.SetTrackedObjectPos`
  (params (ObjectPos :type "Vector Structure") (IsGood :type Boolean))
  (if (`self.Activated`)
    (set `self.TrackedObjectPos` ObjectPos)
    (`self.StartTracking`)))

(event `/Game/Blueprints/StandardReciver/BI_Reciver.SetTracking`
  (params (Tracking :type Boolean))
  (set `self.Tracking` Tracking))

(event `StartTracking`
  (set `self.StartTrackedPosition` (`Actor.K2_GetActorLocation` (`self.GetOwner`)))
  (`self.IsTracking`)
  (`self.Update Distance`))

(event `IsTracking`
  (if (`self.Activated`)
    (if (`self.Tracking`)
      (`self.PlayLight`)
      (`self.Play Rumble`)
      (`self.Play Sound`)
      (`self.PlayRotation`)
      (`KismetSystemLibrary.Delay` (`self.Distance`))
      (`self.IsTracking`))))

(event `Update Distance`
  (if (`self.Tracking`)
    (set `self.Distance` (`self.CalculateDistance`))
    (`KismetSystemLibrary.Delay` (`GameplayStatics.GetWorldDeltaSeconds`))
    (`self.Update Distance`)))

(event `Play Sound`
  (if true
    (`GameplayStatics.PlaySound2D` "/Game/Audio/Detector/Beep3.Beep3" 0.5 1.0 0.0 null null)))

(event `Play Rumble`
  (`GameplayStatics.SpawnForceFeedbackAtLocation` "/Game/Blueprints/Rumble/FfeTest.FfeTest" (0.0 0.0 0.0) (struct) false 1.0 0.0 null))

(event `PlayRotation`
  (message `/Game/Blueprints/Detector/BI_Detector.StartSpinning` (`self.GetOwner`) (`self.Distance`)))

(event `Play CameraShake`)

(event `PlayLight`
  (message `/Game/Blueprints/Detector/BI_Detector.LampOff` (`self.GetOwner`))
  (`KismetSystemLibrary.Delay` 0.2)
  (message `/Game/Blueprints/Detector/BI_Detector.LampOn` (`self.GetOwner`)))

(fn `CalculateDistance`
  (returns (`Distance left in %` :type "Float (double-precision)"))
  (return (/ (`KismetMathLibrary.Vector_Distance` (`Actor.K2_GetActorLocation` (`self.GetOwner`)) (`self.TrackedObjectPos`)) (`KismetMathLibrary.Vector_Distance` (`self.StartTrackedPosition`) (`self.TrackedObjectPos`)))))