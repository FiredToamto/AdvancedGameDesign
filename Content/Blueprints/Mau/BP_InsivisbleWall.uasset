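; An invisible boundary volume that sends the player back to the respawn point when they touch it.
; On overlap with the player character, it plays a 2D beep, disables input and pauses message checking on the player's AC_LineTraceChecker component.
; After a short delay it moves the character to the BP_Respawn actor, resumes and resets the checker message, and restores input.
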(event `self.Box.OnComponentBeginOverlap`
  (params (OverlappedComponent :type "PrimitiveComponent Object Reference") (OtherActor :type "Actor Object Reference") (OtherComp :type "PrimitiveComponent Object Reference") (OtherBodyIndex :type Integer) (bFromSweep :type Boolean) (SweepResult :type "HitResult Structure (by ref)"))
  (bind _returnvalue (`GameplayStatics.GetPlayerCharacter` 0))
  (if (== OtherActor _returnvalue)
    (set `self.CheckerComponent` (`self.GetComponentByClass` _returnvalue "/Game/Blueprints/LineTraceChecker/AC_LineTraceChecker.AC_LineTraceChecker_C"))
    (`GameplayStatics.PlaySound2D` "/Game/Audio/Detector/Bip2.Bip2" 1.0 1.0 0.0 null null)
    (`self.DisableInput` (`GameplayStatics.GetPlayerCharacter` 0) (`GameplayStatics.GetPlayerController` 0))
    (message `/Game/Blueprints/LineTraceReciver/BI_LineTraceReciver.SetIsChecking` (`self.CheckerComponent`) false)
    (`KismetSystemLibrary.Delay` 1.5)
    (bind _returnvalue_2 (`GameplayStatics.GetActorOfClass` "/Game/Blueprints/Mau/BP_Respawn.BP_Respawn_C"))
    (`self.K2_SetActorLocation` (`GameplayStatics.GetPlayerCharacter` 0) (`self.K2_GetActorLocation` _returnvalue_2) false false)
    (message `/Game/Blueprints/LineTraceReciver/BI_LineTraceReciver.SetIsChecking` (`self.CheckerComponent`) true)
    (message `/Game/Blueprints/LineTraceReciver/BI_LineTraceReciver.ResetChecker` (`self.CheckerComponent`))
    (`self.EnableInput` (`GameplayStatics.GetPlayerCharacter` 0) (`GameplayStatics.GetPlayerController` 0))))

(fn `UserConstructionScript`)