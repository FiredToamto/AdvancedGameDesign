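; BP_CollisionBox is an actor with two trigger boxes that play repeating force feedback (controller rumble) while overlapped, apparently as a rumble test.
; Each box's begin overlap starts a self-calling Delay loop that spawns the FfeTest effect, one at a fixed interval, the other using the Time variable.
; Both boxes share one Collision flag with no actor filter, so ending overlap on either stops both loops.
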(event `self.Box.OnComponentBeginOverlap`
  (params (OverlappedComponent :type "PrimitiveComponent Object Reference") (OtherActor :type "Actor Object Reference") (OtherComp :type "PrimitiveComponent Object Reference") (OtherBodyIndex :type Integer) (bFromSweep :type Boolean) (SweepResult :type "HitResult Structure (by ref)"))
  (set `self.collision` true)
  (`self.Start`))

(event `self.Box2.OnComponentBeginOverlap`
  (params (OverlappedComponent :type "PrimitiveComponent Object Reference") (OtherActor :type "Actor Object Reference") (OtherComp :type "PrimitiveComponent Object Reference") (OtherBodyIndex :type Integer) (bFromSweep :type Boolean) (SweepResult :type "HitResult Structure (by ref)"))
  (set `self.collision` true)
  (`self.Start2`))

(event `Start`
  (if (`self.collision`)
    (`GameplayStatics.SpawnForceFeedbackAtLocation` "/Game/Blueprints/Rumble/FfeTest.FfeTest" (0.0 0.0 0.0) (struct) false 1.0 0.0 null)
    (`KismetSystemLibrary.Delay` 0.2)
    (`self.Start`)))

(event `Start2`
  (if (`self.collision`)
    (`GameplayStatics.SpawnForceFeedbackAtLocation` "/Game/Blueprints/Rumble/FfeTest.FfeTest" (0.0 0.0 0.0) (struct) false 1.0 0.0 null)
    (`KismetSystemLibrary.Delay` (`self.Time`))
    (`self.Start2`)))

(event `self.Box2.OnComponentEndOverlap`
  (params (OverlappedComponent :type "PrimitiveComponent Object Reference") (OtherActor :type "Actor Object Reference") (OtherComp :type "PrimitiveComponent Object Reference") (OtherBodyIndex :type Integer))
  (set `self.collision` false))

(event `self.Box.OnComponentEndOverlap`
  (params (OverlappedComponent :type "PrimitiveComponent Object Reference") (OtherActor :type "Actor Object Reference") (OtherComp :type "PrimitiveComponent Object Reference") (OtherBodyIndex :type Integer))
  (set `self.collision` false))

(fn `UserConstructionScript`)