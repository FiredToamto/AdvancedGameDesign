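; Detector device that signals a normalized distance through a row of lamps and a spinning propeller.
; Lower distance lights more lamps via threshold branches and spins the propeller faster on Tick, in either direction.
; ChangeChecker flip-flops the lit material between good and bad while timelines flick the lever; SpinnDial turns a three-position dial with static sounds.
; DeactivateLamps stops Tick and switches the lamps off in a staggered sequence.
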(event `/Game/Blueprints/Detector/BI_Detector.LampOn`
  (`PrimitiveComponent.SetMaterial` (`self.GoodLamp`) 0 (`self.CurrentMaterial`)))

(event `self.ReceiveBeginPlay`
  (`PrimitiveComponent.SetMaterial` (`self.Lamp2`) 0 "/Game/Art/Materials/Detector/M_Lamp_Off.M_Lamp_Off")
  (`PrimitiveComponent.SetMaterial` (`self.Lamp3`) 0 "/Game/Art/Materials/Detector/M_Lamp_Off.M_Lamp_Off")
  (`PrimitiveComponent.SetMaterial` (`self.Lamp4`) 0 "/Game/Art/Materials/Detector/M_Lamp_Off.M_Lamp_Off")
  (`PrimitiveComponent.SetMaterial` (`self.Lamp5`) 0 "/Game/Art/Materials/Detector/M_Lamp_Off.M_Lamp_Off")
  (`PrimitiveComponent.SetMaterial` (`self.Lamp6`) 0 "/Game/Art/Materials/Detector/M_Lamp_Off.M_Lamp_Off")
  (`PrimitiveComponent.SetMaterial` (`self.GoodLamp`) 0 "/Game/Art/Materials/Detector/M_Lamp_Off.M_Lamp_Off")
  (`SceneComponent.K2_SetRelativeRotation` (`self.Lever`) (`KismetMathLibrary.MakeRotator` 0.0 -40.0) false false))

(event `/Game/Blueprints/Detector/BI_Detector.LampOff`
  (`PrimitiveComponent.SetMaterial` (`self.GoodLamp`) 0 "/Game/Art/Materials/Detector/M_Lamp_Off.M_Lamp_Off"))

(event `/Game/Blueprints/Detector/BI_Detector.SpinnDial`
  (params (DialNumber :type Integer))
  (if (== (`self.LastDial`) 1)
    (if (== DialNumber 2)
      (set `self.LastDial` DialNumber)
      (`GameplayStatics.PlaySound2D` "/Game/Audio/Detector/Dial/Static1.Static1" 1.0 1.0 0.0 null null)
      (`|ExecutionSequence`
        (:`then_0`
          (bind (_direction _dialspin) (`Timeline|RotateDial120-240` :`NewTime` 0.25 :!via `Stop` :!label _label)
            (:`Update`
              (`SceneComponent.K2_SetRelativeRotation` (`self.Dial`) (`KismetMathLibrary.MakeRotator` 90.0 _dialspin) false false))))
        (:`then_1`
          (bind (_direction_2 _dialspin_2) (`Timeline|RotateDial240-360` :`NewTime` 0.25 :!via `Stop` :!label _label_2)
            (:`Update`
              (`SceneComponent.K2_SetRelativeRotation` (`self.Dial`) (`KismetMathLibrary.MakeRotator` 90.0 _dialspin_2) false false))))
        (:`then_2`
          (bind (_direction_3 _dialspin_3) (`Timeline|RotateDial0-120` :`NewTime` 0.25 :!via `PlayFromStart` :!label _label_3)
            (:`Update`
              (`SceneComponent.K2_SetRelativeRotation` (`self.Dial`) (`KismetMathLibrary.MakeRotator` 90.0 _dialspin_3) false false)))))
      (else
        (set `self.LastDial` DialNumber)
        (`GameplayStatics.PlaySound2D` "/Game/Audio/Detector/Dial/Static3.Static3" 1.0 1.0 0.0 null null)
        (`|ExecutionSequence`
          (:`then_0`
            (goto _label_3 :!via `Stop`))
          (:`then_1`
            (goto _label :!via `Stop`))
          (:`then_2`
            (goto _label_2 :!via `SetNewTime`))
          (:`then_3`
            (goto _label_2 :!via `Reverse`)))))
    (elif (== (`self.LastDial`) 2)
      (if (== DialNumber 1)
        (set `self.LastDial` DialNumber)
        (`GameplayStatics.PlaySound2D` "/Game/Audio/Detector/Dial/Static2.Static2" 1.0 1.0 0.0 null null)
        (`|ExecutionSequence`
          (:`then_0`
            (goto _label_2 :!via `Stop`))
          (:`then_1`
            (goto _label :!via `Stop`))
          (:`then_2`
            (goto _label_3 :!via `SetNewTime`))
          (:`then_3`
            (goto _label_3 :!via `Reverse`)))
        (else
          (set `self.LastDial` DialNumber)
          (`GameplayStatics.PlaySound2D` "/Game/Audio/Detector/Dial/Static3.Static3" 1.0 1.0 0.0 null null)
          (`|ExecutionSequence`
            (:`then_0`
              (goto _label_3 :!via `Stop`))
            (:`then_1`
              (goto _label_2 :!via `Stop`))
            (:`then_2`
              (goto _label :!via `PlayFromStart`)))))
      (elif (== DialNumber 2)
        (set `self.LastDial` DialNumber)
        (`GameplayStatics.PlaySound2D` "/Game/Audio/Detector/Dial/Static1.Static1" 1.0 1.0 0.0 null null)
        (`|ExecutionSequence`
          (:`then_0`
            (goto _label_3 :!via `Stop`))
          (:`then_1`
            (goto _label_2 :!via `Stop`))
          (:`then_2`
            (goto _label :!via `SetNewTime`))
          (:`then_3`
            (goto _label :!via `Reverse`)))
        (else
          (set `self.LastDial` DialNumber)
          (`GameplayStatics.PlaySound2D` "/Game/Audio/Detector/Dial/Static2.Static2" 1.0 1.0 0.0 null null)
          (`|ExecutionSequence`
            (:`then_0`
              (goto _label_3 :!via `Stop`))
            (:`then_1`
              (goto _label :!via `Stop`))
            (:`then_2`
              (goto _label_2 :!via `PlayFromStart`))))))))

(event `/Game/Blueprints/Mau/BI_Player.ChangeChecker`
  (`/Engine/EditorBlueprintResources/StandardMacros.FlipFlop`
    (:`A`
      (set `self.CurrentMaterial` "/Game/Art/Materials/Detector/M_Lamp_Bad.M_Lamp_Bad")
      (`|ExecutionSequence`
        (:`then_0`
          (bind (_direction _flicklever) (`Timeline|LeverFlick` :`NewTime` 0.25 :!via `Stop` :!label _label_4)
            (:`Update`
              (`SceneComponent.K2_SetRelativeRotation` (`self.Lever`) (`KismetMathLibrary.MakeRotator` 0.0 _flicklever) false false))))
        (:`then_1`
          (goto _label_4))))
    (:`B`
      (set `self.CurrentMaterial` "/Game/Art/Materials/Detector/M_Lamp_Good.M_Lamp_Good")
      (`|ExecutionSequence`
        (:`then_0`
          (goto _label_4 :!via `Stop`))
        (:`then_1`
          (goto _label_4 :!via `SetNewTime`))
        (:`then_2`
          (goto _label_4 :!via `Reverse`))))))

(event `/Game/Blueprints/Detector/BI_Detector.StartSpinning`
  (params (Distance :type "Float (single-precision)") (IsPositive :type Boolean))
  (set `self.CurrentDistance` Distance)
  (set `self.IsPositiveSpin` IsPositive)
  (set `self.PorpellerIsSpinning` true)
  (`self.SetActorTickEnabled` true))

(event `self.ReceiveTick`
  (params (DeltaSeconds :type "Float (single-precision)"))
  (set `self.RotSpeed` (* (`KismetMathLibrary.Lerp` 500.0 0.0 (`self.CurrentDistance`)) 2.0))
  (if (not (`self.IsPositiveSpin`))
    (set `self.RotSpeed` (* (`self.RotSpeed`) -1.0)))
  (`SceneComponent.K2_AddLocalRotation` (`self.Propeller`) (* (`KismetMathLibrary.MakeRotator` 0.0 0.0 (`self.RotSpeed`)) DeltaSeconds) false false))

(event `/Game/Blueprints/Detector/BI_Detector.Lamps`
  (params (Distance :type "Float (single-precision)"))
  (set `self.CurrentDistance` Distance)
  (if (>= (`self.CurrentDistance`) 0.9091)
    (`PrimitiveComponent.SetMaterial` (`self.Lamp11`) 0 (`self.CurrentMaterial`))
    (`PrimitiveComponent.SetMaterial` (`self.Lamp9`) 0 "/Game/Art/Materials/Detector/M_Lamp_Off.M_Lamp_Off")
    (`PrimitiveComponent.SetMaterial` (`self.Lamp8`) 0 "/Game/Art/Materials/Detector/M_Lamp_Off.M_Lamp_Off")
    (`PrimitiveComponent.SetMaterial` (`self.Lamp10`) 0 "/Game/Art/Materials/Detector/M_Lamp_Off.M_Lamp_Off")
    (`PrimitiveComponent.SetMaterial` (`self.Lamp7`) 0 "/Game/Art/Materials/Detector/M_Lamp_Off.M_Lamp_Off")
    (`PrimitiveComponent.SetMaterial` (`self.Lamp6`) 0 "/Game/Art/Materials/Detector/M_Lamp_Off.M_Lamp_Off")
    (`PrimitiveComponent.SetMaterial` (`self.Lamp5`) 0 "/Game/Art/Materials/Detector/M_Lamp_Off.M_Lamp_Off")
    (`PrimitiveComponent.SetMaterial` (`self.Lamp4`) 0 "/Game/Art/Materials/Detector/M_Lamp_Off.M_Lamp_Off")
    (`PrimitiveComponent.SetMaterial` (`self.Lamp3`) 0 "/Game/Art/Materials/Detector/M_Lamp_Off.M_Lamp_Off")
    (`PrimitiveComponent.SetMaterial` (`self.Lamp2`) 0 "/Game/Art/Materials/Detector/M_Lamp_Off.M_Lamp_Off")
    (elif (>= (`self.CurrentDistance`) 0.8182)
      (`PrimitiveComponent.SetMaterial` (`self.Lamp11`) 0 (`self.CurrentMaterial`))
      (`PrimitiveComponent.SetMaterial` (`self.Lamp10`) 0 (`self.CurrentMaterial`))
      (`PrimitiveComponent.SetMaterial` (`self.Lamp9`) 0 "/Game/Art/Materials/Detector/M_Lamp_Off.M_Lamp_Off")
      (`PrimitiveComponent.SetMaterial` (`self.Lamp8`) 0 "/Game/Art/Materials/Detector/M_Lamp_Off.M_Lamp_Off")
      (`PrimitiveComponent.SetMaterial` (`self.Lamp7`) 0 "/Game/Art/Materials/Detector/M_Lamp_Off.M_Lamp_Off")
      (`PrimitiveComponent.SetMaterial` (`self.Lamp6`) 0 "/Game/Art/Materials/Detector/M_Lamp_Off.M_Lamp_Off")
      (`PrimitiveComponent.SetMaterial` (`self.Lamp5`) 0 "/Game/Art/Materials/Detector/M_Lamp_Off.M_Lamp_Off")
      (`PrimitiveComponent.SetMaterial` (`self.Lamp4`) 0 "/Game/Art/Materials/Detector/M_Lamp_Off.M_Lamp_Off")
      (`PrimitiveComponent.SetMaterial` (`self.Lamp3`) 0 "/Game/Art/Materials/Detector/M_Lamp_Off.M_Lamp_Off")
      (`PrimitiveComponent.SetMaterial` (`self.Lamp2`) 0 "/Game/Art/Materials/Detector/M_Lamp_Off.M_Lamp_Off")
      (elif (>= (`self.CurrentDistance`) 0.7273)
        (`PrimitiveComponent.SetMaterial` (`self.Lamp11`) 0 (`self.CurrentMaterial`))
        (`PrimitiveComponent.SetMaterial` (`self.Lamp10`) 0 (`self.CurrentMaterial`))
        (`PrimitiveComponent.SetMaterial` (`self.Lamp9`) 0 (`self.CurrentMaterial`))
        (`PrimitiveComponent.SetMaterial` (`self.Lamp8`) 0 "/Game/Art/Materials/Detector/M_Lamp_Off.M_Lamp_Off")
        (`PrimitiveComponent.SetMaterial` (`self.Lamp7`) 0 "/Game/Art/Materials/Detector/M_Lamp_Off.M_Lamp_Off")
        (`PrimitiveComponent.SetMaterial` (`self.Lamp6`) 0 "/Game/Art/Materials/Detector/M_Lamp_Off.M_Lamp_Off")
        (`PrimitiveComponent.SetMaterial` (`self.Lamp5`) 0 "/Game/Art/Materials/Detector/M_Lamp_Off.M_Lamp_Off")
        (`PrimitiveComponent.SetMaterial` (`self.Lamp4`) 0 "/Game/Art/Materials/Detector/M_Lamp_Off.M_Lamp_Off")
        (`PrimitiveComponent.SetMaterial` (`self.Lamp3`) 0 "/Game/Art/Materials/Detector/M_Lamp_Off.M_Lamp_Off")
        (`PrimitiveComponent.SetMaterial` (`self.Lamp2`) 0 "/Game/Art/Materials/Detector/M_Lamp_Off.M_Lamp_Off")
        (elif (>= (`self.CurrentDistance`) 0.6364)
          (`PrimitiveComponent.SetMaterial` (`self.Lamp11`) 0 (`self.CurrentMaterial`))
          (`PrimitiveComponent.SetMaterial` (`self.Lamp10`) 0 (`self.CurrentMaterial`))
          (`PrimitiveComponent.SetMaterial` (`self.Lamp9`) 0 (`self.CurrentMaterial`))
          (`PrimitiveComponent.SetMaterial` (`self.Lamp8`) 0 (`self.CurrentMaterial`))
          (`PrimitiveComponent.SetMaterial` (`self.Lamp7`) 0 "/Game/Art/Materials/Detector/M_Lamp_Off.M_Lamp_Off")
          (`PrimitiveComponent.SetMaterial` (`self.Lamp6`) 0 "/Game/Art/Materials/Detector/M_Lamp_Off.M_Lamp_Off")
          (`PrimitiveComponent.SetMaterial` (`self.Lamp5`) 0 "/Game/Art/Materials/Detector/M_Lamp_Off.M_Lamp_Off")
          (`PrimitiveComponent.SetMaterial` (`self.Lamp4`) 0 "/Game/Art/Materials/Detector/M_Lamp_Off.M_Lamp_Off")
          (`PrimitiveComponent.SetMaterial` (`self.Lamp3`) 0 "/Game/Art/Materials/Detector/M_Lamp_Off.M_Lamp_Off")
          (`PrimitiveComponent.SetMaterial` (`self.Lamp2`) 0 "/Game/Art/Materials/Detector/M_Lamp_Off.M_Lamp_Off")
          (elif (>= (`self.CurrentDistance`) 0.5455)
            (`PrimitiveComponent.SetMaterial` (`self.Lamp11`) 0 (`self.CurrentMaterial`))
            (`PrimitiveComponent.SetMaterial` (`self.Lamp10`) 0 (`self.CurrentMaterial`))
            (`PrimitiveComponent.SetMaterial` (`self.Lamp9`) 0 (`self.CurrentMaterial`))
            (`PrimitiveComponent.SetMaterial` (`self.Lamp8`) 0 (`self.CurrentMaterial`))
            (`PrimitiveComponent.SetMaterial` (`self.Lamp7`) 0 (`self.CurrentMaterial`))
            (`PrimitiveComponent.SetMaterial` (`self.Lamp6`) 0 "/Game/Art/Materials/Detector/M_Lamp_Off.M_Lamp_Off")
            (`PrimitiveComponent.SetMaterial` (`self.Lamp5`) 0 "/Game/Art/Materials/Detector/M_Lamp_Off.M_Lamp_Off")
            (`PrimitiveComponent.SetMaterial` (`self.Lamp4`) 0 "/Game/Art/Materials/Detector/M_Lamp_Off.M_Lamp_Off")
            (`PrimitiveComponent.SetMaterial` (`self.Lamp3`) 0 "/Game/Art/Materials/Detector/M_Lamp_Off.M_Lamp_Off")
            (`PrimitiveComponent.SetMaterial` (`self.Lamp2`) 0 "/Game/Art/Materials/Detector/M_Lamp_Off.M_Lamp_Off")
            (elif (>= (`self.CurrentDistance`) 0.4546)
              (`PrimitiveComponent.SetMaterial` (`self.Lamp11`) 0 (`self.CurrentMaterial`))
              (`PrimitiveComponent.SetMaterial` (`self.Lamp6`) 0 (`self.CurrentMaterial`))
              (`PrimitiveComponent.SetMaterial` (`self.Lamp10`) 0 (`self.CurrentMaterial`))
              (`PrimitiveComponent.SetMaterial` (`self.Lamp9`) 0 (`self.CurrentMaterial`))
              (`PrimitiveComponent.SetMaterial` (`self.Lamp8`) 0 (`self.CurrentMaterial`))
              (`PrimitiveComponent.SetMaterial` (`self.Lamp7`) 0 (`self.CurrentMaterial`))
              (`PrimitiveComponent.SetMaterial` (`self.Lamp5`) 0 "/Game/Art/Materials/Detector/M_Lamp_Off.M_Lamp_Off")
              (`PrimitiveComponent.SetMaterial` (`self.Lamp4`) 0 "/Game/Art/Materials/Detector/M_Lamp_Off.M_Lamp_Off")
              (`PrimitiveComponent.SetMaterial` (`self.Lamp3`) 0 "/Game/Art/Materials/Detector/M_Lamp_Off.M_Lamp_Off")
              (`PrimitiveComponent.SetMaterial` (`self.Lamp2`) 0 "/Game/Art/Materials/Detector/M_Lamp_Off.M_Lamp_Off")
              (elif (>= (`self.CurrentDistance`) 0.3637)
                (`PrimitiveComponent.SetMaterial` (`self.Lamp11`) 0 (`self.CurrentMaterial`))
                (`PrimitiveComponent.SetMaterial` (`self.Lamp10`) 0 (`self.CurrentMaterial`))
                (`PrimitiveComponent.SetMaterial` (`self.Lamp9`) 0 (`self.CurrentMaterial`))
                (`PrimitiveComponent.SetMaterial` (`self.Lamp8`) 0 (`self.CurrentMaterial`))
                (`PrimitiveComponent.SetMaterial` (`self.Lamp7`) 0 (`self.CurrentMaterial`))
                (`PrimitiveComponent.SetMaterial` (`self.Lamp6`) 0 (`self.CurrentMaterial`))
                (`PrimitiveComponent.SetMaterial` (`self.Lamp5`) 0 (`self.CurrentMaterial`))
                (`PrimitiveComponent.SetMaterial` (`self.Lamp4`) 0 "/Game/Art/Materials/Detector/M_Lamp_Off.M_Lamp_Off")
                (`PrimitiveComponent.SetMaterial` (`self.Lamp3`) 0 "/Game/Art/Materials/Detector/M_Lamp_Off.M_Lamp_Off")
                (`PrimitiveComponent.SetMaterial` (`self.Lamp2`) 0 "/Game/Art/Materials/Detector/M_Lamp_Off.M_Lamp_Off")
                (elif (>= (`self.CurrentDistance`) 0.2728)
                  (`PrimitiveComponent.SetMaterial` (`self.Lamp11`) 0 (`self.CurrentMaterial`))
                  (`PrimitiveComponent.SetMaterial` (`self.Lamp10`) 0 (`self.CurrentMaterial`))
                  (`PrimitiveComponent.SetMaterial` (`self.Lamp9`) 0 (`self.CurrentMaterial`))
                  (`PrimitiveComponent.SetMaterial` (`self.Lamp8`) 0 (`self.CurrentMaterial`))
                  (`PrimitiveComponent.SetMaterial` (`self.Lamp7`) 0 (`self.CurrentMaterial`))
                  (`PrimitiveComponent.SetMaterial` (`self.Lamp6`) 0 (`self.CurrentMaterial`))
                  (`PrimitiveComponent.SetMaterial` (`self.Lamp5`) 0 (`self.CurrentMaterial`))
                  (`PrimitiveComponent.SetMaterial` (`self.Lamp4`) 0 (`self.CurrentMaterial`))
                  (`PrimitiveComponent.SetMaterial` (`self.Lamp3`) 0 "/Game/Art/Materials/Detector/M_Lamp_Off.M_Lamp_Off")
                  (`PrimitiveComponent.SetMaterial` (`self.Lamp2`) 0 "/Game/Art/Materials/Detector/M_Lamp_Off.M_Lamp_Off")
                  (elif (>= (`self.CurrentDistance`) 0.1819)
                    (`PrimitiveComponent.SetMaterial` (`self.Lamp11`) 0 (`self.CurrentMaterial`))
                    (`PrimitiveComponent.SetMaterial` (`self.Lamp10`) 0 (`self.CurrentMaterial`))
                    (`PrimitiveComponent.SetMaterial` (`self.Lamp9`) 0 (`self.CurrentMaterial`))
                    (`PrimitiveComponent.SetMaterial` (`self.Lamp8`) 0 (`self.CurrentMaterial`))
                    (`PrimitiveComponent.SetMaterial` (`self.Lamp7`) 0 (`self.CurrentMaterial`))
                    (`PrimitiveComponent.SetMaterial` (`self.Lamp6`) 0 (`self.CurrentMaterial`))
                    (`PrimitiveComponent.SetMaterial` (`self.Lamp5`) 0 (`self.CurrentMaterial`))
                    (`PrimitiveComponent.SetMaterial` (`self.Lamp4`) 0 (`self.CurrentMaterial`))
                    (`PrimitiveComponent.SetMaterial` (`self.Lamp3`) 0 (`self.CurrentMaterial`))
                    (`PrimitiveComponent.SetMaterial` (`self.Lamp2`) 0 "/Game/Art/Materials/Detector/M_Lamp_Off.M_Lamp_Off")
                    (elif (>= (`self.CurrentDistance`) 0.091)
                      (`PrimitiveComponent.SetMaterial` (`self.Lamp11`) 0 (`self.CurrentMaterial`))
                      (`PrimitiveComponent.SetMaterial` (`self.Lamp10`) 0 (`self.CurrentMaterial`))
                      (`PrimitiveComponent.SetMaterial` (`self.Lamp9`) 0 (`self.CurrentMaterial`))
                      (`PrimitiveComponent.SetMaterial` (`self.Lamp8`) 0 (`self.CurrentMaterial`))
                      (`PrimitiveComponent.SetMaterial` (`self.Lamp7`) 0 (`self.CurrentMaterial`))
                      (`PrimitiveComponent.SetMaterial` (`self.Lamp6`) 0 (`self.CurrentMaterial`))
                      (`PrimitiveComponent.SetMaterial` (`self.Lamp5`) 0 (`self.CurrentMaterial`))
                      (`PrimitiveComponent.SetMaterial` (`self.Lamp4`) 0 (`self.CurrentMaterial`))
                      (`PrimitiveComponent.SetMaterial` (`self.Lamp3`) 0 (`self.CurrentMaterial`))
                      (`PrimitiveComponent.SetMaterial` (`self.Lamp2`) 0 (`self.CurrentMaterial`)))))))))))))

(event `/Game/Blueprints/Detector/BI_Detector.DeactivateLamps`
  (`self.SetActorTickEnabled` false)
  (`PrimitiveComponent.SetMaterial` (`self.GoodLamp`) 0 "/Game/Art/Materials/Detector/M_Lamp_Off.M_Lamp_Off")
  (`KismetSystemLibrary.Delay` 0.1)
  (`PrimitiveComponent.SetMaterial` (`self.Lamp2`) 0 "/Game/Art/Materials/Detector/M_Lamp_Off.M_Lamp_Off")
  (`KismetSystemLibrary.Delay` 0.1)
  (`PrimitiveComponent.SetMaterial` (`self.Lamp3`) 0 "/Game/Art/Materials/Detector/M_Lamp_Off.M_Lamp_Off")
  (`KismetSystemLibrary.Delay` 0.1)
  (`PrimitiveComponent.SetMaterial` (`self.Lamp4`) 0 "/Game/Art/Materials/Detector/M_Lamp_Off.M_Lamp_Off")
  (`KismetSystemLibrary.Delay` 0.1)
  (`PrimitiveComponent.SetMaterial` (`self.Lamp5`) 0 "/Game/Art/Materials/Detector/M_Lamp_Off.M_Lamp_Off")
  (`KismetSystemLibrary.Delay` 0.1)
  (`PrimitiveComponent.SetMaterial` (`self.Lamp6`) 0 "/Game/Art/Materials/Detector/M_Lamp_Off.M_Lamp_Off")
  (`KismetSystemLibrary.Delay` 0.1)
  (`PrimitiveComponent.SetMaterial` (`self.Lamp7`) 0 "/Game/Art/Materials/Detector/M_Lamp_Off.M_Lamp_Off")
  (`KismetSystemLibrary.Delay` 0.1)
  (`PrimitiveComponent.SetMaterial` (`self.Lamp8`) 0 "/Game/Art/Materials/Detector/M_Lamp_Off.M_Lamp_Off")
  (`KismetSystemLibrary.Delay` 0.1)
  (`PrimitiveComponent.SetMaterial` (`self.Lamp9`) 0 "/Game/Art/Materials/Detector/M_Lamp_Off.M_Lamp_Off")
  (`KismetSystemLibrary.Delay` 0.1)
  (`PrimitiveComponent.SetMaterial` (`self.Lamp10`) 0 "/Game/Art/Materials/Detector/M_Lamp_Off.M_Lamp_Off")
  (`KismetSystemLibrary.Delay` 0.1)
  (`PrimitiveComponent.SetMaterial` (`self.Lamp11`) 0 "/Game/Art/Materials/Detector/M_Lamp_Off.M_Lamp_Off"))

(fn `CalcNewRotAndStartRot`
  (bind (_returnvalue_roll _returnvalue_pitch _returnvalue_yaw) (`KismetMathLibrary.BreakRotator` (`SceneComponent.K2_GetComponentRotation` (`self.Propeller`))))
  (set `self.StartPos` (`SceneComponent.K2_GetComponentRotation` (`self.Propeller`)))
  (set `self.NewPos` (`KismetMathLibrary.MakeRotator` _returnvalue_roll _returnvalue_pitch (+ _returnvalue_yaw 360.0))))

(fn `GetDetector`
  (returns (BpDetectorRef :type "/Game/Blueprints/Detector/BP_Detector Object Reference"))
  (return self))

(fn `UserConstructionScript`)