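; Receiver component that gives force feedback rumble, pulsing faster and stronger as its owner nears a tracked position.
; Setting the position records the owner's start location and, while Tracking is on, runs two self-recalling Delay loops.
; A per-frame loop computes remaining distance as a fraction of the start distance and picks a stepped intensity.
; The pulse loop scales its interval by that fraction; light and camera shake events are empty, and sound is never called.
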(event `/Game/Blueprints/StandardReciver/BI_Reciver.SetTrackedObjectPos`
  (params (ObjectPos :type "Vector Structure") (IsGood :type Boolean))
  (set `self.TrackedObjectPos` ObjectPos)
  (`self.StartTracking`))

(event `/Game/Blueprints/StandardReciver/BI_Reciver.SetTracking`
  (params (Tracking :type Boolean))
  (set `self.Tracking` Tracking))

(event `StartTracking`
  (set `self.StartTrackedPosition` (`Actor.K2_GetActorLocation` (`self.GetOwner`)))
  (`self.IsTracking`)
  (`self.Update Distance`))

(event `IsTracking`
  (if (`self.Tracking`)
    (`KismetSystemLibrary.Delay` (`KismetMathLibrary.FClamp` (* (`self.Distance`) 2.0) 0.2 2.0))
    (`self.Play Rumble`)
    (`self.IsTracking`)))

(event `Update Distance`
  (if (`self.Tracking`)
    (set `self.Distance` (`self.CalculateDistance`))
    (`self.RumbleMultiplier`)
    (`KismetSystemLibrary.Delay` (`GameplayStatics.GetWorldDeltaSeconds`))
    (`self.Update Distance`)))

(event `Play Sound`
  (`GameplayStatics.PlaySound2D` "/Game/Audio/Firstperson/FirstPersonTemplateWeaponFire02.FirstPersonTemplateWeaponFire02" 0.5 1.0 0.0 null null))

(event `Play Rumble`
  (if (`self.Isrumble`)
    (`GameplayStatics.SpawnForceFeedbackAtLocation` "/Game/Blueprints/Rumble/FfeTest.FfeTest" (0.0 0.0 0.0) (struct) false (`self.rumbleMulti`) 0.0 null)))

(event `PlayLight`)

(event `Play CameraShake`)

(fn `CalculateDistance`
  (returns (`Distance left in %` :type "Float (double-precision)"))
  (return (/ (`KismetMathLibrary.Vector_Distance` (`Actor.K2_GetActorLocation` (`self.GetOwner`)) (`self.TrackedObjectPos`)) (`KismetMathLibrary.Vector_Distance` (`self.StartTrackedPosition`) (`self.TrackedObjectPos`)))))

(fn `RumbleMultiplier`
  (if (>= (`self.Distance`) 0.6)
    (`KismetSystemLibrary.PrintString` "1 multi")
    (set `self.rumbleMulti` 0.5)
    (elif (>= (`self.Distance`) 0.3)
      (`KismetSystemLibrary.PrintString` "2 multi")
      (set `self.rumbleMulti` 1.0)
      (elif (>= (`self.Distance`) 0.0)
        (`KismetSystemLibrary.PrintString` "3 multi")
        (set `self.rumbleMulti` 2.5)))))