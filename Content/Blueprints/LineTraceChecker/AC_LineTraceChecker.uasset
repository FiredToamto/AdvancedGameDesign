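; Actor component that periodically scans around its owner for objects and reports the nearest visible one to the owner's AC_LineTraceReciver component.
; A self-repeating delayed loop fires eight horizontal debug-drawn traces along fixed world directions, then keeps hits within 45 degrees of the owner's forward vector.
; The closest hit drives receiver messages for looking state, position, distance and tracking.
; Losing all hits or calling the reset events clears tracking.
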(event `self.ReceiveBeginPlay`
  ;[0 1 0.9451] Save reciever component
  (set `self.RecieverComponent` (`Actor.GetComponentByClass` (`self.GetOwner`) "/Game/Blueprints/LineTraceReciver/AC_LineTraceReciver.AC_LineTraceReciver_C"))
  (set `self.LatestHitActor` (`self.ActorReset`))
  ;[1 0 0.8309] Start to line trace
  (`self.CheckForObjects`))

(event `CheckForObjects`
  ;[1 1 1] Should it check?
  (if (`self.IsChecking`)
    ;[1 0 0.02512] Raycast in 8 directions
    (`self.RaycastFixedDistance` (750.0 0.0 0.0))
    (`self.RaycastFixedDistance` (-750.0 0.0 0.0))
    (`self.RaycastFixedDistance` (0.0 750.0 0.0))
    (`self.RaycastFixedDistance` (0.0 -750.0 0.0))
    (`self.RaycastFixedDistance` (-525.0 -525.0 0.0))
    (`self.RaycastFixedDistance` (525.0 525.0 0.0))
    (`self.RaycastFixedDistance` (-525.0 525.0 0.0))
    (`self.RaycastFixedDistance` (525.0 -525.0 0.0))
    ;[1 0.9289 0] If it got any hits
    (if (> (`KismetArrayLibrary.Array_Length` (`self.Distances`)) 0)
      ;[0.2543 1 0] If any hit is in sight
      (bind _inrange (`self.CheckIfObjectInSight`))
      (if _inrange
        ;[0.5795 0.2586 1] Set is looking
        (message `/Game/Blueprints/LineTraceReciver/BI_LineTraceReciver.NotLooking` (`self.RecieverComponent`) false)
        ;[1 0.4099 0.6132] Check closest distance
        (bind (_closestleangth _array_index) (`self.CheckDistances` (`self.Distances`)))
        ;[1 0.9856 0.3176] If it was first hit
        (if (== (`self.ActorReset`) (`self.LatestHitActor`))
          (bind _output (`|GetArrayItem` (`self.HitActors`) _array_index))
          (set `self.LatestHitActor` _output)
          (bind _output_2 (`|GetArrayItem` (`self.Locations`) _array_index))
          ;[1 0.4533 0.2926] Set new tracked object
          (message `/Game/Blueprints/StandardReciver/BI_Reciver.SetTrackedObjectPos` (`self.RecieverComponent`) _output_2 false)
          ;[0.3297 0.6319 1] Send closest distance for calculation
          (set `self.ClosestRange` _closestleangth)
          (message `/Game/Blueprints/LineTraceReciver/BI_LineTraceReciver.SendDistance` (`self.RecieverComponent`) _closestleangth)
          ;[0.2292 0.2292 0.2292] Activate tracking
          (message `/Game/Blueprints/StandardReciver/BI_Reciver.SetTracking` (`self.RecieverComponent`) true)
          (else
            ;[0.4394 1 0.6077] If the latest hit is the same as before
            (if (== _output (`self.LatestHitActor`))
              ;[0.7655 0.291 1] If closest range is nearer than before
              (if (< _closestleangth (`self.ClosestRange`))
                (set `self.ClosestRange` _closestleangth))
              (message `/Game/Blueprints/LineTraceReciver/BI_LineTraceReciver.SendDistance` (`self.RecieverComponent`) _closestleangth)
              (else
                (set `self.ClosestRange` _closestleangth)))
            ;[1 0.4533 0.2926] Set new tracked object
            (message `/Game/Blueprints/StandardReciver/BI_Reciver.SetTrackedObjectPos` (`self.RecieverComponent`) _output_2 false)))
        ;[0.3694 1 0.3778] Reset arrays
        (`KismetArrayLibrary.Array_Clear` (`self.Distances`))
        (`KismetArrayLibrary.Array_Clear` (`self.Locations`))
        (`KismetArrayLibrary.Array_Clear` (`self.HitActors`))
        (`KismetSystemLibrary.Delay` (`self.CheckTimer`))
        ;[0 0.02998 1] REPEAT
        (`self.CheckForObjects`)
        (else
          ;[0 0.04694 1] If not in sight then is not looking (REPEAT)
          (message `/Game/Blueprints/LineTraceReciver/BI_LineTraceReciver.NotLooking` (`self.RecieverComponent`) true)
          (`KismetSystemLibrary.Delay` (`self.CheckTimer`))
          (`self.CheckForObjects`)))
      (else
        ;[0.4773 0 1] Don't reset values if there was no hit
        (if (not (== (`self.ActorReset`) (`self.LatestHitActor`)))
          ;[0 1 0.2102] Reset values
          (message `/Game/Blueprints/StandardReciver/BI_Reciver.SetTracking` (`self.RecieverComponent`) false :!label _label)
          (set `self.LatestHitActor` (`self.ActorReset`))
          (set `self.ClosestRange` 0.0)
          (`KismetSystemLibrary.Delay` (`self.CheckTimer`))
          ;[0 0.02998 1] REPEAT
          (`self.CheckForObjects`)
          (else
            (`KismetSystemLibrary.Delay` (`self.CheckTimer`))
            ;[0 0.02998 1] REPEAT
            (`self.CheckForObjects`)))))))

(event `/Game/Blueprints/LineTraceReciver/BI_LineTraceReciver.SetIsChecking`
  (params (ChangeCheckingTo :type Boolean))
  ;[0.5605 1 0.7698] Set if Checking or not
  (set `self.IsChecking` ChangeCheckingTo)
  (goto _label))

(event `/Game/Blueprints/LineTraceReciver/BI_LineTraceReciver.ResetChecker`
  ;[1 0.6784 0.2226] Reset checker
  (goto _label))

(fn `CheckDistances`
  (params (Distances :type "Array of Float (double-precision)"))
  (returns (ClosestLeangth :type "Float (double-precision)") (`Array Index` :type Integer))
  (locals (Closest :type "Float (double-precision)" :default 10000.0) (ClosestArrayIndex :type Integer))
  (for (_array_element _array_index) Distances
    (if (< _array_element (`local.Closest`))
      ;[1 1 1] Save the closest distance hit
      (set `local.Closest` _array_element)
      (set `local.ClosestArrayIndex` _array_index)))
  (return (`local.Closest`) (`local.ClosestArrayIndex`)))

(fn `CheckIfObjectInSight`
  (returns (InRange :type Boolean))
  (locals (ToRemove :type "Array of Integer") (TempDistance :type "Array of Float (double-precision)") (TempLocations :type "Array of Vector Structure") (TempHitActors :type "Array of Actor Object Reference"))
  (bind _returnvalue (`self.GetOwner`))
  (for (_array_element _array_index) (`self.Locations`)
    (if (< (`KismetMathLibrary.DegAcos` (`KismetMathLibrary.Dot_VectorVector` (`KismetMathLibrary.Normal` (- _array_element (`Actor.K2_GetActorLocation` _returnvalue))) (`Actor.GetActorForwardVector` _returnvalue))) 45.0)
      ;[1 0.2366 0.1968] Save info about hits in vision
      (`KismetArrayLibrary.Array_Add` (`local.TempDistance`) (`|GetArrayItem` (`self.Distances`) _array_index))
      (`KismetArrayLibrary.Array_Add` (`local.TempLocations`) (`|GetArrayItem` (`self.Locations`) _array_index))
      (`KismetArrayLibrary.Array_Add` (`local.TempHitActors`) (`|GetArrayItem` (`self.HitActors`) _array_index))))
  ;[0.8094 1 0.3379] Renew arrays with correct info and check if there is anything left
  (set `self.Distances` (`local.TempDistance`))
  (set `self.Locations` (`local.TempLocations`))
  (set `self.HitActors` (`local.TempHitActors`))
  (return (> (`KismetArrayLibrary.Array_Length` (`self.Distances`)) 0)))

(fn `GetDetector`
  (returns (BpDetectorRef :type "/Game/Blueprints/Detector/BP_Detector Object Reference"))
  (return null))

(fn `Raycast Fixed Distance Fixed Rotation`
  (params (EndDistance :type "Vector Structure") (Distance :type "Float (double-precision)") (Offset :type "Float (double-precision)"))
  (locals (ForwardX :type "Float (double-precision)") (ForwardY :type "Float (double-precision)") (LocOffset :type "Float (double-precision)") (LocDistance :type "Float (double-precision)"))
  (bind _returnvalue (`Actor.K2_GetActorLocation` (`self.GetOwner`)))
  (bind _returnvalue_2 (`Actor.K2_GetActorLocation` (`self.GetOwner`)))
  (bind _returnvalue_3 (`Actor.K2_GetActorLocation` (`self.GetOwner`)))
  (bind _returnvalue_4 (`Actor.K2_GetActorLocation` (`self.GetOwner`)))
  ;[1 1 1] Scrapped
  (set `local.LocDistance` Distance)
  (set `local.LocOffset` Offset)
  (set `local.ForwardY` (.y (`KismetMathLibrary.GetForwardVector` (`Actor.K2_GetActorRotation` (`self.GetOwner`)))))
  (set `local.ForwardX` (.x (`KismetMathLibrary.GetForwardVector` (`Actor.K2_GetActorRotation` (`self.GetOwner`)))))
  (if (and (> (`local.ForwardX`) 0.0) (> (`local.ForwardY`) 0.0))
    (`KismetSystemLibrary.LineTraceSingle` :`Start` _returnvalue_2 :`End` (+ _returnvalue_2 (* (`KismetMathLibrary.MakeVector` (`local.ForwardX`) (- (`local.ForwardY`) (`local.LocOffset`))) (`local.LocDistance`))) :`TraceChannel` "TraceTypeQuery3" :`DrawDebugType` "ForDuration" :`DrawTime` 0.1)
    (elif (and (> 0.0 (`local.ForwardX`)) (> 0.0 (`local.ForwardY`)))
      (`KismetSystemLibrary.LineTraceSingle` :`Start` _returnvalue_4 :`End` (+ _returnvalue_4 (* (`KismetMathLibrary.MakeVector` (- (`local.ForwardX`) (`local.LocOffset`)) (`local.ForwardY`)) (`local.LocDistance`))) :`TraceChannel` "TraceTypeQuery3" :`DrawDebugType` "ForDuration" :`DrawTime` 0.1)
      (elif (and (> 0.0 (`local.ForwardX`)) (> (`local.ForwardY`) 0.0))
        (`KismetSystemLibrary.LineTraceSingle` :`Start` _returnvalue :`End` (+ _returnvalue (* (`KismetMathLibrary.MakeVector` (`local.ForwardX`) (- (`local.ForwardY`) (`local.LocOffset`))) (`local.LocDistance`))) :`TraceChannel` "TraceTypeQuery3" :`DrawDebugType` "ForDuration" :`DrawTime` 0.1)
        (else
          (bind (_outhit _returnvalue_5) (`KismetSystemLibrary.LineTraceSingle` :`Start` _returnvalue_3 :`End` (+ _returnvalue_3 (* (`KismetMathLibrary.MakeVector` (- (`local.ForwardX`) (`local.LocOffset`)) (`local.ForwardY`)) (`local.LocDistance`))) :`TraceChannel` "TraceTypeQuery3" :`DrawDebugType` "ForDuration" :`DrawTime` 0.1))))))
  (if _returnvalue_5
    (bind (_bblockinghit _binitialoverlap _time _distance _location _impactpoint _normal _impactnormal _physmat _hitactor) (`GameplayStatics.BreakHitResult` _outhit))
    (`KismetArrayLibrary.Array_Add` (`self.Distances`) _distance)
    (`KismetArrayLibrary.Array_Add` (`self.Locations`) _location)
    (`KismetArrayLibrary.Array_Add` (`self.HitActors`) _hitactor))
  (return))

(fn `RaycastFixedDistance`
  (params (EndDistance :type "Vector Structure"))
  (bind _returnvalue (`self.GetOwner`))
  (bind _returnvalue_2 (`Actor.K2_GetActorLocation` _returnvalue))
  ;[1 0.3074 0.4477] Linetrace based upon distances and rotation
  (bind (_outhit _returnvalue_3) (`KismetSystemLibrary.LineTraceSingle` :`Start` _returnvalue_2 :`End` (+ EndDistance (+ _returnvalue_2 (`Actor.GetActorForwardVector` _returnvalue))) :`TraceChannel` "TraceTypeQuery3" :`DrawDebugType` "ForDuration" :`DrawTime` 0.1))
  ;[1 0.9992 0.3139] Save info if hit
  (if _returnvalue_3
    (bind (_bblockinghit _binitialoverlap _time _distance _location _impactpoint _normal _impactnormal _physmat _hitactor) (`GameplayStatics.BreakHitResult` _outhit))
    (`KismetArrayLibrary.Array_Add` (`self.Distances`) _distance)
    (`KismetArrayLibrary.Array_Add` (`self.Locations`) _location)
    (`KismetArrayLibrary.Array_Add` (`self.HitActors`) _hitactor))
  (return))